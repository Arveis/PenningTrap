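; BP_Generator is an interactable generator that sends the player to the next level once they carry enough antimatter.
; Overlapping its box with BP_PlayerBase shows a text prompt and opens a gate on the Interaction input, and leaving hides and closes both.
; Each accepted press plays the Reaktor sound, then opens NextLevel if the player's Antimatter is non-zero and meets AntimatterRequired.
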(event `self.ReceiveBeginPlay`
  (`self.EnableInput` (`GameplayStatics.GetPlayerController` 0)))

(event `InputAction|Interaction`
  (params (Key :type "Key Structure"))
  (:`Pressed`
    (`/Engine/EditorBlueprintResources/StandardMacros.Gate` true :!label _label
      (:`Exit`
        (`GameplayStatics.SpawnSound2D` "/Game/Audio/SFX/Reaktor.Reaktor" 1.0 1.0 0.0 null)
        (`GameplayStatics.PlaySound2D` "/Game/Audio/SFX/Reaktor.Reaktor" 1.0 1.0 0.0 null null)
        (bind _antimatter (`/Game/Blueprints/BP_PlayerBase.Antimatter` (stale `self.Box.OnComponentBeginOverlap` _asbp_player_base)))
        (if (and (>= _antimatter (`self.Antimatter Required`)) (!= _antimatter 0.0))
          (`GameplayStatics.OpenLevel` (`self.Next Level`)))))))

(event `self.Box.OnComponentBeginOverlap`
  (params (OverlappedComponent :type "PrimitiveComponent Object Reference") (OtherActor :type "Actor Object Reference") (OtherComp :type "PrimitiveComponent Object Reference") (OtherBodyIndex :type Integer) (bFromSweep :type Boolean) (SweepResult :type "HitResult Structure (by ref)"))
  (bind _asbp_player_base (cast `/Game/Blueprints/BP_PlayerBase` OtherActor))
  (`SceneComponent.SetVisibility` (`self.TextRender`) true false)
  (goto _label :!via `Open`))

(event `self.Box.OnComponentEndOverlap`
  (params (OverlappedComponent :type "PrimitiveComponent Object Reference") (OtherActor :type "Actor Object Reference") (OtherComp :type "PrimitiveComponent Object Reference") (OtherBodyIndex :type Integer))
  (`SceneComponent.SetVisibility` (`self.TextRender`) false false)
  (goto _label :!via `Close`))

(fn `UserConstructionScript`)