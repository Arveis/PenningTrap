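; BP_EnemyBase is an enemy base actor that moves along a two-point path and can drop antimatter loot.
; The construction script feeds Location1 and Location2 to InterpToMovement as relative control points and sets its travel time from DurationTime.
; SpawnLoot spawns a BP_AntimatterPickUp at the root's world transform, then destroys the enemy.
; The event graph holds no active logic, and nothing here calls SpawnLoot.
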(fn `SpawnLoot`
  (`|SpawnActorFromClass` "/Game/Blueprints/BP_AntimatterPickUp.BP_AntimatterPickUp_C" (`SceneComponent.K2_GetComponentToWorld` (`self.DefaultSceneRoot`)) "Undefined" "OverrideRootScale" null null)
  (`self.K2_DestroyActor`))

(fn `UserConstructionScript`
  (bind _interptomovement (`self.InterpToMovement`))
  (set `InterpToMovementComponent.ControlPoints` (`|MakeArray` (make `InterpControlPoint` (`self.Location1`)) (make `InterpControlPoint` (`self.Location2`))) _interptomovement)
  (set `InterpToMovementComponent.Duration` (`self.DurationTime`) _interptomovement))