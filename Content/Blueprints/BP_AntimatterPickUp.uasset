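; BP_AntimatterPickUp is a pickup that grants antimatter to the player and then destroys itself.
; On BeginPlay, a timeline lerps the actor's X and Z scale from their initial values toward a fixed target, with Y held at zero.
; Each update of that timeline also plays a second timeline that animates the point light's intensity.
; Box overlap with a BP_PlayerBase calls AddAntimatter before destroying the actor.
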(event `self.ReceiveBeginPlay`
  (bind (_returnvalue_x _returnvalue_y _returnvalue_z) (`KismetMathLibrary.BreakVector` (`self.GetActorScale3D`)))
  (set `self.Scale X` _returnvalue_x)
  (set `self.Scale Z` _returnvalue_z)
  (bind (_direction _scale) (`Timeline|Timeline_0`)
    (:`Update`
      (`self.SetActorScale3D` (`KismetMathLibrary.MakeVector` (`KismetMathLibrary.Lerp` (`self.Scale X`) 1.5 _scale) 0.0 (`KismetMathLibrary.Lerp` (`self.Scale Z`) 1.5 _scale)))
      (bind (_direction_2 _newtrack_0) (`Timeline|Timeline_1`)
        (:`Update`
          (`LightComponent.SetIntensity` (`self.PointLight`) (* _newtrack_0 600.0)))))))

(event `self.Box.OnComponentBeginOverlap`
  (params (OverlappedComponent :type "PrimitiveComponent Object Reference") (OtherActor :type "Actor Object Reference") (OtherComp :type "PrimitiveComponent Object Reference") (OtherBodyIndex :type Integer) (bFromSweep :type Boolean) (SweepResult :type "HitResult Structure (by ref)"))
  (bind _asbp_player_base (cast `/Game/Blueprints/BP_PlayerBase` OtherActor))
  (`/Game/Blueprints/BP_PlayerBase.AddAntimatter` _asbp_player_base)
  (`self.K2_DestroyActor`))

(fn `UserConstructionScript`)